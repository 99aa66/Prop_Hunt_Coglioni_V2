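; Game mode for a multiplayer session, with an empty new-player override and a logout handler that removes departing controllers from PlayerControllers.
; A disconnected, never-executed chain holds the lobby logic: register players, debounce with a retriggerable delay, then read session settings.
; Once the session is full, that chain kicks surplus players, updates the session and possesses a spawned C_Player per controller at index-named player starts.
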(event `self.HandleStartingNewPlayer`
  (params (NewPlayer :type "PlayerController Object Reference")))

(event `self.K2_OnLogout`
  (params (ExitingController :type "Controller Object Reference"))
  (bind _asplayer_controller (cast `PlayerController` ExitingController))
  (`KismetArrayLibrary.Array_RemoveItem` (`self.playerControllers`) _asplayer_controller))

(fn `UserConstructionScript`)