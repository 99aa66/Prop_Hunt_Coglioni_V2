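; Hider player character for Prop Hunt that disguises itself as props it shoots and can un-prop or play a random taunt.
; The shot component's mesh name looks up DT_Props; a matching row becomes CurrentProp.
; CurrentProp's RepNotify toggles the character mesh, applies the prop mesh, resizes the capsule and spawns a poof on authority.
; Un-propping sets an empty prop with default capsule size; taunts multicast one of seven attached sounds.
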(event `self.SR_Shoot`
  ;[0.05098 0.05098 0.05098] Become a prop
  (bind (_hitactor _hitcomponent) (`self.Shoot`))
  (`self.BecomeProp` _hitcomponent))

(event `InputAction|Un-prop`
  (params (Key :type "Key Structure"))
  ;[0.05098 0.05098 0.05098] Un-prop by setting the Current prop to contain no static mesh
  (:`Pressed`
    (`self.SR_Un-prop`)))

(event `InputAction|Taunt`
  (params (Key :type "Key Structure"))
  ;[0.05098 0.05098 0.05098] Taunt
  (:`Pressed`
    (`self.SR_Taunt`)))

(event `SR_Taunt`
  ;[0.05098 0.05098 0.05098] Taunt
  (`self.Do_RandomTaunt`))

(event `SR_Un-prop`
  ;[0.05098 0.05098 0.05098] Un-prop by setting the Current prop to contain no static mesh
  (set `self.Current_Prop` (make `/Game/PropHunt/Blueprints/Core/Gameplay/Data/S_Prop` "" null 90.0 35.0)))

(fn `BecomeProp`
  (params (HitComponent :type "Object Object Reference"))
  (bind _returnvalue (`KismetSystemLibrary.GetDisplayName` HitComponent))
  ;[0.05098 0.05098 0.05098] Checks if the Static Mesh is an available prop, then if it's found in our Props Datatable we set it as our Current Prop
  (bind _returnvalue_2 (`|GetDataTableRow` "/Game/PropHunt/Blueprints/Core/Gameplay/Data/DT_Props.DT_Props" (`KismetStringLibrary.Conv_StringToName` (`KismetStringLibrary.Replace` (`KismetStringLibrary.RightChop` _returnvalue (`KismetStringLibrary.FindSubstring` _returnvalue " " false true)) " ")))
    (:`then`
      (set `self.Current_Prop` _returnvalue_2))))

(fn `Do_RandomTaunt`
  (switch `int` (`KismetMathLibrary.RandomIntegerInRange` 0 6)
    (:`0`
      (`self.MC_SpawnSoundAttached` "/Game/PropHunt/Assets/Audio/Cues/SC_Taunt1.SC_Taunt1"))
    (:`1`
      (`self.MC_SpawnSoundAttached` "/Game/PropHunt/Assets/Audio/Cues/SC_Taunt2.SC_Taunt2"))
    (:`2`
      (`self.MC_SpawnSoundAttached` "/Game/PropHunt/Assets/Audio/Cues/SC_Taunt3.SC_Taunt3"))
    (:`3`
      (`self.MC_SpawnSoundAttached` "/Game/PropHunt/Assets/Audio/Cues/SC_Taunt4.SC_Taunt4"))
    (:`4`
      (`self.MC_SpawnSoundAttached` "/Game/PropHunt/Assets/Audio/Cues/SC_Taunt5.SC_Taunt5"))
    (:`5`
      (`self.MC_SpawnSoundAttached` "/Game/PropHunt/Assets/Audio/Cues/SC_Taunt6.SC_Taunt6"))
    (:`6`
      (`self.MC_SpawnSoundAttached` "/Game/PropHunt/Assets/Audio/Cues/SC_Taunt7.SC_Taunt7"))))

(fn `OnRep_Current_Prop`
  (bind (_current_prop_name _current_prop_staticmesh _current_prop_capsule_halfheight _current_prop_capsule_radius) (break `/Game/PropHunt/Blueprints/Core/Gameplay/Data/S_Prop` (`self.Current_Prop`)))
  ;[0.05098 0.05098 0.05098] Switch our character's Mesh visibility based on wether or not the current prop name is empty
  (`SceneComponent.SetVisibility` (`self.Mesh`) (`KismetStringLibrary.IsEmpty` _current_prop_name) true)
  ;[0.05098 0.05098 0.05098] Sets the Static Mesh and adjusts the Capsule size and the Static Mesh location to fit correctly in the new Capsule size.
  (`StaticMeshComponent.SetStaticMesh` (`self.StaticMesh`) _current_prop_staticmesh)
  (`CapsuleComponent.SetCapsuleRadius` (`self.CapsuleComponent`) _current_prop_capsule_radius true)
  (`CapsuleComponent.SetCapsuleHalfHeight` (`self.CapsuleComponent`) _current_prop_capsule_halfheight true)
  (`SceneComponent.K2_SetRelativeLocation` (`self.StaticMesh`) (`KismetMathLibrary.MakeVector` 0.0 0.0 (* _current_prop_capsule_halfheight -1.0)) false false)
  ;[0.05098 0.05098 0.05098] Spawns a Poof particle each time we become a prop or un-prop
  (`/Engine/EditorBlueprintResources/ActorMacros.Switch Has Authority`
    (:`Authority`
      (`self.SR_SpawnPoof`))))

(fn `UserConstructionScript`
  (`parent.UserConstructionScript`))